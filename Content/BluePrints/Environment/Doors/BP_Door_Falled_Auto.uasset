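; BP_Door_Falled_Auto is an automatic drop-down door that pitches open when BP_ThirdPersonCharacter enters its collision box and closes on exit.
; One timeline, played forward or in reverse, rotates DoorDownRotator up to MaxDoorOpenAngle and updates IsDoorOpen from its finishing direction.
; An InProgress guard ignores requests mid-swing without queuing them, so an early exit can leave the door open.
; The construction script pre-rotates doors flagged IsDoorOpen.
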(event OnComponentBeginOverlap(BoxCollision)
  (params (OverlappedComponent :type Primitive%20Component%20Object%20Reference) (OtherActor :type Actor%20Object%20Reference) (OtherComp :type Primitive%20Component%20Object%20Reference) (OtherBodyIndex :type Integer) (bFromSweep :type Boolean) (SweepResult :type Hit%20Result%20Structure%20%28by%20ref%29))
  (Utilities|Casting|CastToBP_ThirdPersonCharacter OtherActor)
  (CallFunction|OpenDoor))

(event OnComponentEndOverlap(BoxCollision)
  (params (OverlappedComponent :type Primitive%20Component%20Object%20Reference) (OtherActor :type Actor%20Object%20Reference) (OtherComp :type Primitive%20Component%20Object%20Reference) (OtherBodyIndex :type Integer))
  (Utilities|Casting|CastToBP_ThirdPersonCharacter OtherActor)
  (CallFunction|CloseDoor))

(event Custom|OpenDoor
  ;[1 1 1] Открывание двери с таймлайном и проверками
  (if (not (Variables|Default|GetInProgress))
    (if (not (Variables|DoorConfigue|GetIsDoorOpen))
      (bind (_direction _openprogression) (Timeline|Timeline_0 PlayFromStart)
        (:Update
          (Variables|Default|SetInProgress true)
          (Transformation|SetRelativeRotation (Variables|Default|GetDoorDownRotator) (Math|Rotator|MakeRotator 0.0 (* (Variables|DoorConfigue|GetMaxDoorOpenAngle) _openprogression) 0.0) false false))
        (:Finished
          (Variables|Default|SetInProgress false)
          (switch Utilities|FlowControl|Switch|SwitchonETimelineDirection _direction
            (:Forward
              (Variables|DoorConfigue|SetIsDoorOpen true))
            (:Backward
              (Variables|DoorConfigue|SetIsDoorOpen false))))))))

(event Custom|CloseDoor
  ;[1 1 1] Открывание двери с таймлайном и проверками
  (if (not (Variables|Default|GetInProgress))
    (if (Variables|DoorConfigue|GetIsDoorOpen)
      (bind (_direction _openprogression) (Timeline|Timeline_0 ReverseFromEnd)
        (:Update
          (Variables|Default|SetInProgress true)
          (Transformation|SetRelativeRotation (Variables|Default|GetDoorDownRotator) (Math|Rotator|MakeRotator 0.0 (* (Variables|DoorConfigue|GetMaxDoorOpenAngle) _openprogression) 0.0) false false))
        (:Finished
          (Variables|Default|SetInProgress false)
          (switch Utilities|FlowControl|Switch|SwitchonETimelineDirection _direction
            (:Forward
              (Variables|DoorConfigue|SetIsDoorOpen true))
            (:Backward
              (Variables|DoorConfigue|SetIsDoorOpen false))))))))

(event EventBeginPlay)

(event Collision|EventActorBeginOverlap
  (params (OtherActor :type Actor%20Object%20Reference)))

(event EventTick
  (params (DeltaSeconds :type Float%20%28single-precision%29)))

(fn ConstructionScript
  (Transformation|AddRelativeRotation (Variables|Default|GetDoorDownRotator) (Math|Rotator|MakeRotator 0.0 (Math|Float|SelectFloat (Variables|DoorConfigue|GetMaxDoorOpenAngle) 0.0 (Variables|DoorConfigue|GetIsDoorOpen)) 0.0) false false))