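; Falling door that swings on its pitch axis between closed and open, toggled through a box collision trigger.
; The trigger toggles it when the third-person character leaves the box, or when any other actor enters.
; One timeline scales the max angle onto the door rotator and plays in reverse to close, with an in-progress flag blocking retriggers.
; The construction script pre-rotates the door if it is set to start open.
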(event OnComponentBeginOverlap(BoxCollision)
  (params (OverlappedComponent :type Primitive%20Component%20Object%20Reference) (OtherActor :type Actor%20Object%20Reference) (OtherComp :type Primitive%20Component%20Object%20Reference) (OtherBodyIndex :type Integer) (bFromSweep :type Boolean) (SweepResult :type Hit%20Result%20Structure%20%28by%20ref%29))
  (Utilities|Casting|CastToBP_ThirdPersonCharacter OtherActor
    (:CastFailed
      (if (Variables|Default|GetIsDoorOpen)
        (CallFunction|CloseDoor)
        (else
          (CallFunction|OpenDoor))))))

(event OnComponentEndOverlap(BoxCollision)
  (params (OverlappedComponent :type Primitive%20Component%20Object%20Reference) (OtherActor :type Actor%20Object%20Reference) (OtherComp :type Primitive%20Component%20Object%20Reference) (OtherBodyIndex :type Integer))
  (Utilities|Casting|CastToBP_ThirdPersonCharacter OtherActor)
  (if (Variables|Default|GetIsDoorOpen)
    (CallFunction|CloseDoor)
    (else
      (CallFunction|OpenDoor))))

(event EventBeginPlay
  (|CallParentFunction) ; This node is disabled and will not be called.\nDrag off pins to build functionality.
)

(event Collision|EventActorBeginOverlap
  (params (OtherActor :type Actor%20Object%20Reference))
  (|CallParentFunction OtherActor) ; This node is disabled and will not be called.\nDrag off pins to build functionality.
)

(event EventTick
  (params (DeltaSeconds :type Float%20%28single-precision%29))
  (|CallParentFunction DeltaSeconds) ; This node is disabled and will not be called.\nDrag off pins to build functionality.
)

(event EventOpenDoor
  ;[1 1 1] Door, rotate on axis Y on angle 90
  (if (not (Variables|Default|GetInProgress))
    (if (not (Variables|Default|GetIsDoorOpen))
      (bind (_direction _openprogression) (Timeline|DoorFallingTimeLine PlayFromStart)
        (:Update
          (Variables|Default|SetInProgress true)
          (Transformation|SetRelativeRotation (Variables|Default|GetDoorRotator) (Math|Rotator|MakeRotator 0.0 (* (Variables|Default|GetMaxDoorOpenAngle) _openprogression) 0.0) false false))
        (:Finished
          (Variables|Default|SetInProgress false)
          (switch Utilities|FlowControl|Switch|SwitchonETimelineDirection _direction
            (:Forward
              (Variables|Default|SetIsDoorOpen true))
            (:Backward
              (Variables|Default|SetIsDoorOpen false))))))))

(event EventCloseDoor
  ;[1 1 1] Door, rotate on axis Y on angle 90
  (if (not (Variables|Default|GetInProgress))
    (if (Variables|Default|GetIsDoorOpen)
      (bind (_direction _openprogression) (Timeline|DoorFallingTimeLine ReverseFromEnd)
        (:Update
          (Variables|Default|SetInProgress true)
          (Transformation|SetRelativeRotation (Variables|Default|GetDoorRotator) (Math|Rotator|MakeRotator 0.0 (* (Variables|Default|GetMaxDoorOpenAngle) _openprogression) 0.0) false false))
        (:Finished
          (Variables|Default|SetInProgress false)
          (switch Utilities|FlowControl|Switch|SwitchonETimelineDirection _direction
            (:Forward
              (Variables|Default|SetIsDoorOpen true))
            (:Backward
              (Variables|Default|SetIsDoorOpen false))))))))

(fn ConstructionScript
  (Transformation|AddRelativeRotation (Variables|Default|GetDoorRotator) (Math|Rotator|MakeRotator 0.0 (Math|Float|SelectFloat (Variables|Default|GetMaxDoorOpenAngle) 0.0 (Variables|Default|GetIsDoorOpen)) 0.0) false false))