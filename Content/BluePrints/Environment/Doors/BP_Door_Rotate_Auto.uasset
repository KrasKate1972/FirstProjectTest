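; Automatic rotating door that opens when the third-person character enters its box collision and closes when it leaves.
; A timeline plays forward or in reverse, driving DoorRotator yaw up to MaxDoorOpenAngle and setting IsDoorOpen from its direction on finish.
; InProgress makes open and close requests ignored mid-swing, with no retry afterwards.
; The construction script pre-rotates the door when IsDoorOpen is set.
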(event OnComponentBeginOverlap(BoxCollision)
  (params (OverlappedComponent :type Primitive%20Component%20Object%20Reference) (OtherActor :type Actor%20Object%20Reference) (OtherComp :type Primitive%20Component%20Object%20Reference) (OtherBodyIndex :type Integer) (bFromSweep :type Boolean) (SweepResult :type Hit%20Result%20Structure%20%28by%20ref%29))
  (Utilities|Casting|CastToBP_ThirdPersonCharacter OtherActor)
  (CallFunction|OpenDoor))

(event OnComponentEndOverlap(BoxCollision)
  (params (OverlappedComponent :type Primitive%20Component%20Object%20Reference) (OtherActor :type Actor%20Object%20Reference) (OtherComp :type Primitive%20Component%20Object%20Reference) (OtherBodyIndex :type Integer))
  (Utilities|Casting|CastToBP_ThirdPersonCharacter OtherActor)
  (CallFunction|CloseDoor))

(event Custom|OpenDoor
  ;[1 1 1] Открывание двери с таймлайном и проверками
  (if (not (Variables|Default|GetInProgress))
    (if (not (Variables|DoorConfigure|GetIsDoorOpen))
      (bind (_direction _openprogression) (Timeline|DoorTimeLine PlayFromStart)
        (:Update
          (Variables|Default|SetInProgress true)
          (Transformation|SetRelativeRotation (Variables|Default|GetDoorRotator) (Math|Rotator|MakeRotator 0.0 0.0 (* (Variables|DoorConfigure|GetMaxDoorOpenAngle) _openprogression)) false false))
        (:Finished
          (Variables|Default|SetInProgress false)
          (switch Utilities|FlowControl|Switch|SwitchonETimelineDirection _direction
            (:Forward
              (Variables|DoorConfigure|SetIsDoorOpen true))
            (:Backward
              (Variables|DoorConfigure|SetIsDoorOpen false))))))))

(event Custom|CloseDoor
  ;[1 1 1] Открывание двери с таймлайном и проверками
  (if (not (Variables|Default|GetInProgress))
    (if (Variables|DoorConfigure|GetIsDoorOpen)
      (bind (_direction _openprogression) (Timeline|DoorTimeLine ReverseFromEnd)
        (:Update
          (Variables|Default|SetInProgress true)
          (Transformation|SetRelativeRotation (Variables|Default|GetDoorRotator) (Math|Rotator|MakeRotator 0.0 0.0 (* (Variables|DoorConfigure|GetMaxDoorOpenAngle) _openprogression)) false false))
        (:Finished
          (Variables|Default|SetInProgress false)
          (switch Utilities|FlowControl|Switch|SwitchonETimelineDirection _direction
            (:Forward
              (Variables|DoorConfigure|SetIsDoorOpen true))
            (:Backward
              (Variables|DoorConfigure|SetIsDoorOpen false))))))))

(event Collision|EventActorBeginOverlap
  (params (OtherActor :type Actor%20Object%20Reference)))

(event EventTick
  (params (DeltaSeconds :type Float%20%28single-precision%29)))

(fn ConstructionScript
  (Transformation|AddRelativeRotation (Variables|Default|GetDoorRotator) (Math|Rotator|MakeRotator 0.0 0.0 (Math|Float|SelectFloat (Variables|DoorConfigure|GetMaxDoorOpenAngle) 0.0 (Variables|DoorConfigure|GetIsDoorOpen))) false false))