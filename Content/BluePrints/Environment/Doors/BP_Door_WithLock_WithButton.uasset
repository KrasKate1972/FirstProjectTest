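; BP_Door_WithLock_WithButton is a child door Blueprint that adds a lock and a colored lock-status light.
; The OpenDoor override calls the parent only when IsDoorLocked is false, while CloseDoor always passes through to the parent.
; SwitchLock toggles the lock and refreshes LightLockIndicator, shown red when locked and green when unlocked.
; The construction script also updates the indicator, so it matches the initial lock state.
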(event EventBeginPlay
  (|CallParentFunction) ; This node is disabled and will not be called.\nDrag off pins to build functionality.
)

(event Collision|EventActorBeginOverlap
  (params (OtherActor :type Actor%20Object%20Reference))
  (|CallParentFunction OtherActor) ; This node is disabled and will not be called.\nDrag off pins to build functionality.
)

(event EventTick
  (params (DeltaSeconds :type Float%20%28single-precision%29))
  (|CallParentFunction DeltaSeconds) ; This node is disabled and will not be called.\nDrag off pins to build functionality.
)

(event EventOpenDoor
  ;[1 1 1 1 12] Добавление проверки статуса на "замке" в родительские установки
  (if (not (Variables|DoorConfigure|GetIsDoorLocked))
    (|CallParentFunction)))

(event EventCloseDoor
  (|CallParentFunction))

(fn ConstructionScript
  (|CallParentFunction)
  (CallFunction|UpdateDoorLockIndication))

(fn SwitchLock
  (Variables|DoorConfigure|SetIsDoorLocked (not (Variables|DoorConfigure|GetIsDoorLocked)))
  (CallFunction|UpdateDoorLockIndication))

(fn UpdateDoorLockIndication
  (Rendering|Components|Light|SetLightColor (Variables|Default|GetLightLockIndicator) (Math|Color|SelectColor "(R=1.000000,G=0.020612,B=0.040508,A=1.000000)" "(R=0.230659,G=0.833333,B=0.000000,A=1.000000)" (Variables|DoorConfigure|GetIsDoorLocked)) true))