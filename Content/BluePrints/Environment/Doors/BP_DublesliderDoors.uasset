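; Double sliding door actor that reacts to BP_ThirdPersonCharacter entering and leaving its BoxCollision.
; Overlap events call OpenDoor and CloseDoor, which check InProgress and IsDoorOpen before playing or reversing TimelineSliderDoor.
; The timeline lerps DoorSliderA along Y, while DoorSliderB's offset is multiplied by zero.
; Nodes that update both state flags are disconnected, so neither flag changes at runtime.
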(event OnComponentBeginOverlap(BoxCollision)
  (params (OverlappedComponent :type Primitive%20Component%20Object%20Reference) (OtherActor :type Actor%20Object%20Reference) (OtherComp :type Primitive%20Component%20Object%20Reference) (OtherBodyIndex :type Integer) (bFromSweep :type Boolean) (SweepResult :type Hit%20Result%20Structure%20%28by%20ref%29))
  (Utilities|Casting|CastToBP_ThirdPersonCharacter OtherActor)
  (CallFunction|OpenDoor))

(event OnComponentEndOverlap(BoxCollision)
  (params (OverlappedComponent :type Primitive%20Component%20Object%20Reference) (OtherActor :type Actor%20Object%20Reference) (OtherComp :type Primitive%20Component%20Object%20Reference) (OtherBodyIndex :type Integer))
  (Utilities|Casting|CastToBP_ThirdPersonCharacter OtherActor)
  (CallFunction|CloseDoor))

(event Custom|OpenDoor
  ;[1 1 1] Открывание двери с таймлайном и проверками
  (if (not (Variables|Default|GetInProgress))
    (if (not (Variables|DoorConfigue|GetIsDoorOpen))
      (bind _openprogression (Timeline|TimelineSliderDoor PlayFromStart)
        (:Update
          (Utilities|FlowControl|Sequence
            (:then_0
              (Transformation|SetRelativeLocation (Variables|Default|GetDoorSlider_A) (Math|Vector|MakeVector 0.0 (Math|Float|Lerp 0.0 1e+02 _openprogression) 0.0) false false))
            (:then_1
              (Transformation|SetRelativeLocation (Variables|Default|GetDoorSlider_B) (Math|Vector|MakeVector 0.0 (* 0.0 (Math|Float|Lerp 0.0 1e+02 _openprogression)) 0.0) false false))))))))

(event Custom|CloseDoor
  ;[1 1 1] Открывание двери с таймлайном и проверками
  (if (not (Variables|Default|GetInProgress))
    (if (Variables|DoorConfigue|GetIsDoorOpen)
      (bind _openprogression (Timeline|TimelineSliderDoor ReverseFromEnd)
        (:Update
          (Utilities|FlowControl|Sequence
            (:then_0
              (Transformation|SetRelativeLocation (Variables|Default|GetDoorSlider_A) (Math|Vector|MakeVector 0.0 (Math|Float|Lerp 0.0 1e+02 _openprogression) 0.0) false false))
            (:then_1
              (Transformation|SetRelativeLocation (Variables|Default|GetDoorSlider_B) (Math|Vector|MakeVector 0.0 (* 0.0 (Math|Float|Lerp 0.0 1e+02 _openprogression)) 0.0) false false))))))))

(event EventBeginPlay)

(event Collision|EventActorBeginOverlap
  (params (OtherActor :type Actor%20Object%20Reference)))

(event EventTick
  (params (DeltaSeconds :type Float%20%28single-precision%29)))

(fn ConstructionScript)