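; BP_Tooltip is a level-placed tooltip that shows a text message while a Character stands inside its box.
; The construction script applies the exposed box extent, raises the box by its Z extent, then sets the text's position and message.
; Actor overlap events cast to Character, unhide or hide the text, and store or clear the CharacterInBox reference, which is not read in these graphs.
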(event EventBeginPlay)

(event Collision|EventActorBeginOverlap
  (params (OtherActor :type Actor%20Object%20Reference))
  ;[1 1 1] Появление текста при вхождении в периметр Box
  ;;[1 1 1 1 10] Эта нода проверяет кто столкнулся, и если это Character, то проигрывает след. ноду.
  (bind _ascharacter (Utilities|Casting|CastToCharacter OtherActor))
  ;;[1 1 1] ПОявляется видимый текст
  (Variables|Default|SetCharacterIn%20Box _ascharacter)
  (Development|SetHiddeninGame (Variables|Default|GetTooltipText) false false))

(event EventTick
  (params (DeltaSeconds :type Float%20%28single-precision%29)))

(event Collision|EventActorEndOverlap
  (params (OtherActor :type Actor%20Object%20Reference))
  ;[1 1 1] Исчезновение текста при выходе из периметра Box
  (Utilities|Casting|CastToCharacter OtherActor)
  (Variables|Default|SetCharacterIn%20Box 0)
  (Development|SetHiddeninGame (Variables|Default|GetTooltipText) true false))

(fn ConstructionScript
  ;[1 1 1] Text  on the level in the boxcollision.
  ;;[1 1 1] Этот блок отвечает за появление текста
  (Components|Box|SetBoxExtent (Variables|Default|GetBoxCollision) (Variables|ToolTipSettings|GetBox%20Extent) true)
  (Transformation|SetRelativeLocation (Variables|Default|GetBoxCollision) (Math|Vector|MakeVector 0.0 0.0 (.Z (Math|Vector|BreakVector (Variables|ToolTipSettings|GetBox%20Extent)))) false false)
  ;;[1 1 1] Эта часть твечает за слежение текста за персонажем
  (Transformation|SetRelativeLocation (Variables|Default|GetTooltipText) (Variables|ToolTipSettings|GetTooltipTextCollision) false false)
  (Rendering|Components|TextRender|SetText (Variables|Default|GetTooltipText) (Variables|ToolTipSettings|GetToolTipTextMessage)))