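; BP_Toombler is an interactable toggle switch that flips the lock state of an assigned list of doors.
; Overlapping it shows a text prompt and allows Interact, which calls SwitchOn or SwitchOff based on the current state.
; A single timeline plays forward or backward to slide the stick mesh, then updates the state and calls SwitchLock on each door.
; The construction script offsets the stick to match the initial state.
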(event Custom|SwitchOn
  (if (not (Variables|Default|GetInProgress))
    (if (not (Variables|Default|GetIsTumblerOn))
      (bind (_direction _tumblertimline) (Timeline|Timeline_0 PlayFromStart)
        (:Update
          (Variables|Default|SetInProgress true)
          (Transformation|SetRelativeLocation (Variables|Default|GetToomblerStickMesh) (Math|Vector|MakeVector 0.0 (* (Variables|Default|GetMaxStickOffset) _tumblertimline) 0.0) false false))
        (:Finished
          (Variables|Default|SetInProgress false)
          (switch Utilities|FlowControl|Switch|SwitchonETimelineDirection _direction
            (:Forward
              (Variables|Default|SetIsTumblerOn true))
            (:Backward
              (Variables|Default|SetIsTumblerOn false)))
          (CallFunction|DoorsLockswitch))))))

(event Custom|SwitchOff
  (if (not (Variables|Default|GetInProgress))
    (if (Variables|Default|GetIsTumblerOn)
      (bind (_direction _tumblertimline) (Timeline|Timeline_0 ReverseFromEnd)
        (:Update
          (Variables|Default|SetInProgress true)
          (Transformation|SetRelativeLocation (Variables|Default|GetToomblerStickMesh) (Math|Vector|MakeVector 0.0 (* (Variables|Default|GetMaxStickOffset) _tumblertimline) 0.0) false false))
        (:Finished
          (Variables|Default|SetInProgress false)
          (switch Utilities|FlowControl|Switch|SwitchonETimelineDirection _direction
            (:Forward
              (Variables|Default|SetIsTumblerOn true))
            (:Backward
              (Variables|Default|SetIsTumblerOn false)))
          (CallFunction|DoorsLockswitch))))))

(event EventBeginPlay
  (Rendering|SetVisibility (Variables|Default|GetTextRender) false false))

(event Collision|EventActorBeginOverlap
  (params (OtherActor :type Actor%20Object%20Reference))
  (Rendering|SetVisibility (Variables|Default|GetTextRender) true false)
  (Variables|Default|SetIsReadyToInteract true))

(event EventTick
  (params (DeltaSeconds :type Float%20%28single-precision%29)))

(event Collision|EventActorEndOverlap
  (params (OtherActor :type Actor%20Object%20Reference))
  (Rendering|SetVisibility (Variables|Default|GetTextRender) false false)
  (Variables|Default|SetIsReadyToInteract false))

(fn ConstructionScript
  (Transformation|AddRelativeLocation (Variables|Default|GetToomblerStickMesh) (Math|Vector|MakeVector 0.0 (Math|Float|SelectFloat (Variables|Default|GetMaxStickOffset) 0.0 (Variables|Default|GetIsTumblerOn)) 0.0) false false))

(fn DoorsLockswitch
  (if (Utilities|Array|IsValidIndex (Variables|Default|GetDoors%20to%20Lockswitch))
    (for _array_element (Variables|Default|GetDoors%20to%20Lockswitch)
      (Default|SwitchLock _array_element))))

(fn Interact
  ;[1 1 1] Переключение тумблера в противоположное положение
  (if (Variables|Default|GetIsReadyToInteract)
    (if (Variables|Default|GetIsTumblerOn)
      (CallFunction|SwitchOff)
      (return true)
      (else
        (CallFunction|Switchon)
        (return true)))
    (else
      (return false))))