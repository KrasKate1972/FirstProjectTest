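; Trigger Blueprint that toggles the locks on a set of doors when the player character overlaps it.
; On overlap it runs the parent handler, then checks that OverlapedActor is valid and is a BP_ThirdPersonCharacter.
; It then calls SwitchDoorsLocks, which loops over DoorsToLockswitch and calls SwitchLock on each door.
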(event EventBeginPlay
  (|CallParentFunction) ; This node is disabled and will not be called.\nDrag off pins to build functionality.
)

(event Collision|EventActorBeginOverlap
  (params (OtherActor :type Actor%20Object%20Reference))
  (|CallParentFunction OtherActor)
  (bind _overlapedactor (Variables|Default|GetOverlapedActor)
    (:then
      ;[1 1 1 1 14] Эта нода проверяет, что перед нами наш игрок
      (Utilities|Casting|CastToBP_ThirdPersonCharacter _overlapedactor)
      (CallFunction|SwitchDoorsLocks))
    (:else)))

(event EventTick
  (params (DeltaSeconds :type Float%20%28single-precision%29))
  (|CallParentFunction DeltaSeconds) ; This node is disabled and will not be called.\nDrag off pins to build functionality.
)

(fn ConstructionScript
  (|CallParentFunction))

(fn SwitchDoorsLocks
  (for _array_element (Variables|Default|GetDoorsToLockswitch)
    (Default|SwitchLock _array_element)))