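; BP_TestA is a Blueprint learning sandbox with Russian notes on events, functions and basic nodes.
; BeginPlay fires a color-coded debug print event, then calls NewFunction0 twice around a delay, branching into pure and impure math helpers that feed back into print events.
; The Construction Script writes MyName to a TextRender so it shows in the editor.
; Disconnected snippets demonstrate loops, containers, structs, comparisons and an enum traffic-light cycle, but never run.
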(event Custom|PositiveChackEvent
  ;[1 1 1] Кастомная функция (существует только в EventGraph
  (Development|PrintString (Utilities|String|Append "Positivity is  " (Utilities|String|ToString(Boolean) (CallFunction|SuperPositivePureFunction))) true false "(R=1.000000,G=0.984032,B=0.112136,A=1.000000)"))

(event Custom|CustomEvent_0
  (params (NewParam :type Boolean) (NewParam2 :type Integer) (NewParam4 :type Float%20%28single-precision%29) (NewParam3 :type Name))
  ;[1 1 1] Кастомная функция (существует только в EventGraph
  ;;[1 1 1] Создана в эвентграфе, в деталях добавлены инпуты. Это событие.
  ;;[1 1 1 1 16] Вызов функции: первый раз вызывается prins string  цвета fols (галочки в new param нет), второй раз - true
  (Development|PrintString (Utilities|String|Append "Bool = " (Utilities|String|ToString(Boolean) NewParam) "Float = " (Utilities|String|ToString(Float) NewParam4) " !") true false (Math|Color|SelectColor "(R=0.087307,G=1.000000,B=0.209715,A=1.000000)" "(R=1.000000,G=0.000000,B=0.098099,A=1.000000)" NewParam) 5.0))

(event Collision|EventActorBeginOverlap
  (params (OtherActor :type Actor%20Object%20Reference)))

(event EventTick
  (params (DeltaSeconds :type Float%20%28single-precision%29))
  ;[1 1 1] Написание длительности отрисовки каждого тика на уровне (изолированное написание)
)

(event EventBeginPlay
  ;[1 1 1] Кастомная функция (существует только в EventGraph
  ;;[0.3385 0.3385 0.3385 1 9] отсылка к событию, которое создано на  CustomEvent_0. Будет проигрываться каждый раз, когда код будт попадать сюда.
  (CallFunction|CustomEvent0 false 0 0.0 "None")
  ;;[0.3385 0.3385 0.3385 1 9] отсылка к событию, которое создано на  CustomEvent_0. Будет проигрываться каждый раз, когда код будт попадать сюда.
  (CallFunction|CustomEvent0 true 0 0.0 "None")
  ;;[0.4792 0.4792 0.4792 1 12] У функции, созданой в функциях есть и вход, и выход!!!
  (Test|NewFunction0 "None" (Utilities|Array|MakeArray true) 2)
  (Utilities|FlowControl|Delay 2.0)
  (Test|NewFunction0 "None" (Utilities|Array|MakeArray false) 9))

(fn ConstructionScript
  ;[1 1 1] Подпись объекта уровне с именем объекта (может быть и в Event graf, но с Event begin play. Но тогда именование будет видно только при проигрывании уровня, а не в редакторе). Причем, если использовать Get display name +self,+ объединить Format Text через return value and name, то будет писаться не имя переменной (My name), а имя актора на уровне.
  (Rendering|Components|TextRender|SetText (Variables|Default|GetTextRender) (Utilities|Text|FormatText "My name is {Name} " (Variables|Test|GetMyName))))

(fn NewFunction0
  (params (InName :type Name) (InArray :type Array%20of%20Booleans) (InInt :type Integer))
  ;[1 1 1] Все, что относится к функции, называется РЕАЛИЗАЦИЕЙ функции
  (Utilities|FlowControl|Sequence
    (:then_0)
    (:then_1)
    (:then_2)
    (:then_3
      (if (Utilities|Array|Get(acopy) InArray)
        (bind _output_get (LocalVariables|SetL_Int (* InInt 5)))
        (if (.Success (Test|MultbyFivePure _output_get))
          (bind _output_get_2 (LocalVariables|SetL_Int (.Result (Test|MultbyFivePure _output_get))))
          ;;[1 1 1] Не чистая функция
          (bind _result (Test|AddFiveNotPure _output_get_2))
          (bind _output_get_3 (LocalVariables|SetL_Int _result))
          (CallFunction|CustomEvent0 (Utilities|Array|Get(acopy) InArray) _output_get_3 (Math|Conversions|ToFloat(Integer) (LocalVariables|GetL_Int)) InName)
          (CallFunction|PositiveChackEvent)
          (return (LocalVariables|GetL_Int)))
        (else
          (CallFunction|CustomEvent0 (Utilities|Array|Get(acopy) InArray) 0 (Math|Conversions|ToFloat(Integer) InInt) InName)
          (return (LocalVariables|GetL_Int)))))))

(fn AddFiveNotPure
  (params (InParav :type Integer))
  ;[1 1 1] Локальная функция - НЕ Pure - ей нужно подключение к потоку
  (return (+ InParav 5) 0))

(fn MultbyFivePure
  (params (In%20Param :type Integer))
  ;[1 1 1] Маленькая локальная функция Pure, сделанная в Functions. К ней можно обращаться в EventGraph. ей не нужно подключение к потоку.
  (return (* In%20Param 5) true))

(fn SuperPositivePureFunction
  (return true))